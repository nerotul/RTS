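; BP_RTSPlayerController is the RTS player controller that owns the pause menu and gameplay UI.
; BeginPlay creates both widgets, starts the pause menu collapsed and passes itself to the gameplay widget as its owner controller.
; Escape toggles game pause and swaps which widget is visible.
; E runs a console command for Animation Budget Allocator stats; a budget debug command is left unconnected.
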(event `Key|E`
  (params (Key :type "Key Structure"))
  (:`Pressed`
    (`KismetSystemLibrary.ExecuteConsoleCommand` "stat AnimationBudgetAllocator" null)))

(event `self.ReceiveBeginPlay`
  (bind _returnvalue (`|CreateWidget` "/Game/Blueprints/Widgets/WBP_PauseMenu.WBP_PauseMenu_C"))
  (bind _output_get (set `self.PauseWidget` _returnvalue))
  (`UserWidget.AddToViewport` _output_get 0)
  (`Widget.SetVisibility` _output_get "Collapsed")
  (bind _returnvalue_2 (`|CreateWidget` "/Game/Blueprints/Widgets/WBP_Gameplay.WBP_Gameplay_C"))
  (bind _output_get_2 (set `self.GameplayWidget` _returnvalue_2))
  (set `/Game/Blueprints/Widgets/WBP_Gameplay.OwnerController` self _output_get_2)
  (`UserWidget.AddToViewport` _output_get_2 0))

(event `Key|Escape`
  (params (Key :type "Key Structure"))
  (:`Pressed`
    (if (`GameplayStatics.IsGamePaused`)
      (`GameplayStatics.SetGamePaused` false)
      (`Widget.SetVisibility` (`self.PauseWidget`) "Collapsed")
      (`Widget.SetVisibility` (`self.GameplayWidget`) "Visible")
      (else
        (`GameplayStatics.SetGamePaused` true)
        (`Widget.SetVisibility` (`self.PauseWidget`) "Visible")
        (`Widget.SetVisibility` (`self.GameplayWidget`) "Collapsed")))))

(fn `UserConstructionScript`)