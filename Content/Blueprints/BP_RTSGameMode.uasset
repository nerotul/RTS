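; BP_RTSGameMode is the RTS game mode Blueprint that decides when a match ends in victory or defeat.
; CheckGameOverConditions receives the player and enemy unit counts, showing DEFEAT when the player has none, otherwise VICTORY when the enemy has none.
; Either result creates a WBP_GameOver widget with the result text, adds it to the viewport and pauses the game.
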(fn `CheckGameOverConditions`
  (params (PlayersUnitsCount :type Integer) (EnemyUnitsCount :type Integer))
  (if (== PlayersUnitsCount 0)
    (bind _returnvalue (`|CreateWidget` "/Game/Blueprints/Widgets/WBP_GameOver.WBP_GameOver_C"))
    (`TextBlock.SetText` (`/Game/Blueprints/Widgets/WBP_GameOver.TextBlock_GameResult` _returnvalue) "DEFEAT!")
    (`UserWidget.AddToViewport` _returnvalue 0)
    (`GameplayStatics.SetGamePaused` true :!label _label)
    (elif (== EnemyUnitsCount 0)
      (bind _returnvalue_2 (`|CreateWidget` "/Game/Blueprints/Widgets/WBP_GameOver.WBP_GameOver_C"))
      (`TextBlock.SetText` (`/Game/Blueprints/Widgets/WBP_GameOver.TextBlock_GameResult` _returnvalue_2) "VICTORY!")
      (`UserWidget.AddToViewport` _returnvalue_2 0)
      (goto _label))))

(fn `UserConstructionScript`)