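; RTS player controller Blueprint that handles opening and closing the pause menu.
; On BeginPlay it creates a WBP_PauseMenu widget, adds it to the viewport collapsed and keeps a reference in PauseWidget.
; Pressing Escape toggles the game's paused state and switches that same widget between visible and collapsed to match.
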(event `self.ReceiveBeginPlay`
  (bind _returnvalue (`|CreateWidget` "/Game/Blueprints/Widgets/WBP_PauseMenu.WBP_PauseMenu_C"))
  (bind _output_get (set `self.PauseWidget` _returnvalue))
  (`UserWidget.AddToViewport` _output_get 0)
  (`Widget.SetVisibility` _output_get "Collapsed"))

(event `Key|Escape`
  (params (Key :type "Key Structure"))
  (:`Pressed`
    (if (`GameplayStatics.IsGamePaused`)
      (`GameplayStatics.SetGamePaused` false)
      (`Widget.SetVisibility` (`self.PauseWidget`) "Collapsed")
      (else
        (`GameplayStatics.SetGamePaused` true)
        (`Widget.SetVisibility` (`self.PauseWidget`) "Visible")))))

(fn `UserConstructionScript`)