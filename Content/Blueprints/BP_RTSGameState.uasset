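; RTS game state that tracks how many player and enemy units remain alive on the map.
; On BeginPlay it caches BP_RTSGameMode, counts all UnitBase actors by side and hooks each one's unit-death event.
; Each death decrements the matching side's count and passes both totals to the game mode's game-over check.
; Only units present at BeginPlay are counted and bound.
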(event `self.ReceiveBeginPlay`
  (bind _asbp_rtsgame_mode (cast `/Game/Blueprints/BP_RTSGameMode` (`GameplayStatics.GetGameMode`)))
  (set `self.As BP RTSGame Mode` _asbp_rtsgame_mode)
  (bind _outactors (`GameplayStatics.GetAllActorsOfClass` "/Script/RTS.UnitBase"))
  (bind _output_get (set `self.UnitsOnMap` _outactors))
  (for _array_element _output_get
    (if (`UnitBase.bIsPlayersUnit` _array_element)
      (`/Engine/EditorBlueprintResources/StandardMacros.IncrementInt` (`self.PlayersUnitsCount`)
        (:`  `
          _))
      (else
        (`/Engine/EditorBlueprintResources/StandardMacros.IncrementInt` (`self.EnemyUnitsCount`)
          (:`  `
            _))))
    (add `UnitBase.OnUnitDead` _array_element (delegate `OnUnitDead`))))

(event `OnUnitDead`
  (params (bIsPlayersUnit :type Boolean))
  (bind _playersunitscount (`self.PlayersUnitsCount`))
  (bind _enemyunitscount (`self.EnemyUnitsCount`))
  (if bIsPlayersUnit
    (`/Engine/EditorBlueprintResources/StandardMacros.DecrementInt` _playersunitscount
      (:`  `
        _))
    (else
      (`/Engine/EditorBlueprintResources/StandardMacros.DecrementInt` _enemyunitscount
        (:`  `
          _))))
  (`/Game/Blueprints/BP_RTSGameMode.CheckGameOverConditions` (`self.As BP RTSGame Mode`) _playersunitscount _enemyunitscount))

(fn `UserConstructionScript`)