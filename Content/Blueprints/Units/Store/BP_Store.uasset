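; BP_Store is a clickable RTS store where the player buys units.
; On BeginPlay it creates a collapsed WBP_Store widget with itself as owner, which a left click makes visible.
; It binds to death events of units in EnemiesNearby, and when the count reaches zero it shows WBP_StoreHello and pauses the game.
; OnUnitBought increments the player's unit count in BP_RTSGameState.
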(event `self.ReceiveBeginPlay`
  (bind _returnvalue (`|CreateWidget` "/Game/Blueprints/Widgets/WBP_Store.WBP_Store_C"))
  (bind _output_get (set `self.StoreWidget` _returnvalue))
  (set `/Game/Blueprints/Widgets/WBP_Store.Owner` self _output_get)
  (`UserWidget.AddToViewport` _output_get 0)
  (`Widget.SetVisibility` _output_get "Collapsed")
  (bind _asbp_rtsgame_state (cast `/Game/Blueprints/Framework/BP_RTSGameState` (`GameplayStatics.GetGameState`)))
  (set `self.As BP RTSGame State` _asbp_rtsgame_state)
  (for _array_element (`self.EnemiesNearby`)
    (add `UnitBase.OnUnitDead` _array_element (delegate `OnUnitDead_Event_0`))
    (`/Engine/EditorBlueprintResources/StandardMacros.IncrementInt` (`self.EnemiesNearbyCount`))))

(event `OnUnitDead_Event_0`
  (params (bIsPlayersUnit :type Boolean))
  (bind _result (`/Engine/EditorBlueprintResources/StandardMacros.DecrementInt` (`self.EnemiesNearbyCount`))
    (:`  `
      (if (== _result 0)
        (bind _returnvalue (`|CreateWidget` "/Game/Blueprints/Widgets/WBP_StoreHello.WBP_StoreHello_C"))
        (`UserWidget.AddToViewport` _returnvalue 0)
        (`GameplayStatics.SetGamePaused` true)))))

(event `self.ReceiveActorOnClicked`
  (params (ButtonPressed :type "Key Structure"))
  (if (== ButtonPressed "LeftMouseButton")
    (`Widget.SetVisibility` (`self.StoreWidget`) "Visible")))

(event `self.OnUnitBought`
  (`/Engine/EditorBlueprintResources/StandardMacros.IncrementInt` (`/Game/Blueprints/Framework/BP_RTSGameState.PlayersUnitsCount` (`self.As BP RTSGame State`))))

(fn `UserConstructionScript`)