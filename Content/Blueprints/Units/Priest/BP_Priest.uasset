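; Priest unit Blueprint that handles its health bar, fog-of-war reveal and friend/foe markers.
; While alive, player-owned priests trace vertically each tick and paint their collision UV location into two fog render targets through dynamic materials.
; Ability System health changes update the widget bar, which appears for damaged units in enemy sight.
; Construction sets a team decal and a green or red scene-capture-only dot, hidden on death.
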(event `self.ReceiveBeginPlay`
  (`parent.ReceiveBeginPlay`)
  (bind _aswbp_health_bar (cast `/Game/Blueprints/Widgets/WBP_HealthBar` (`WidgetComponent.GetUserWidgetObject` (`self.HealthWidget`))))
  (bind _output_get (set `self.As WBP Health Bar` _aswbp_health_bar))
  (set `/Game/Blueprints/Widgets/WBP_HealthBar.Owner` self _output_get)
  (`AnimationBudgetBlueprintLibrary.EnableAnimationBudget` true)
  (`self.InitFogReveal`)
  (add `self.OnUnitDead` (delegate `OnUnitDead_Event_0`))
  (add `self.OnHealthChanged` (delegate `OnHealthChanged_Event_0`)))

(event `OnUnitDead_Event_0` :!signature `self.OnUnitDead`
  (params (bIsPlayersUnit :type Boolean))
  (`PrimitiveComponent.SetHiddenInSceneCapture` (`self.PaperSprite`) true))

(event `OnHealthChanged_Event_0`
  (`self.UpdateHealthBarPercentage`)
  (`self.TryToggleHealthWidgetVisibility`))

(event `self.ReceiveTick`
  (params (DeltaSeconds :type "Float (single-precision)"))
  (`parent.ReceiveTick` DeltaSeconds)
  (if (`self.bIsAlive`)
    (`self.UpdateFogReveal`)))

(event `self.OnInEnemySight`
  (`self.TryToggleHealthWidgetVisibility`))

(fn `InitFogReveal`
  (locals (NewLocalVar_0 :type "MaterialInstanceDynamic Object Reference"))
  (bind _returnvalue (`KismetMaterialLibrary.CreateDynamicMaterialInstance` "/Game/Blueprints/Fog/M_FogMaterial.M_FogMaterial"))
  (set `self.FogMaterial` _returnvalue)
  (bind _returnvalue_2 (`KismetMaterialLibrary.CreateDynamicMaterialInstance` "/Game/Blueprints/Fog/M_FogRevealMaterial.M_FogRevealMaterial"))
  (set `self.FogRevealMaterial` _returnvalue_2)
  (`KismetRenderingLibrary.ClearRenderTarget2D` "/Game/Blueprints/Fog/FogRender.FogRender")
  (`KismetRenderingLibrary.ClearRenderTarget2D` "/Game/Blueprints/Fog/FogRevealRender.FogRevealRender")
  (`MaterialInstanceDynamic.SetScalarParameterValue` (`self.FogMaterial`) "Size" (`self.Fog Reveal Coeff`)))

(fn `SetFriendFoeSprite`
  (bind _papersprite (`self.PaperSprite`))
  (if (`self.bIsPlayersUnit`)
    (`PaperSpriteComponent.SetSprite` _papersprite "/Game/Assets/Materials/Basic_green_dot_Sprite.Basic_green_dot_Sprite")
    (else
      (`PaperSpriteComponent.SetSprite` _papersprite "/Game/Assets/Materials/Basic_red_dot_Sprite.Basic_red_dot_Sprite"))))

(fn `TryToggleHealthWidgetVisibility`
  (bind _abilitysystemcomponent (`self.AbilitySystemComponent`))
  (bind _healthwidget (`self.HealthWidget`))
  (if (and (`self.bIsAlive`) (`self.bIsUnitInEnemySight`))
    (if (== (/ (`.ReturnValue` (`AbilitySystemBlueprintLibrary.GetFloatAttributeFromAbilitySystemComponent` _abilitysystemcomponent (struct :`AttributeName` "Health" :`Attribute` "/Script/RTS.RTSAttributeSet:Health"))) (`.ReturnValue` (`AbilitySystemBlueprintLibrary.GetFloatAttributeFromAbilitySystemComponent` _abilitysystemcomponent (struct :`AttributeName` "MaxHealth" :`Attribute` "/Script/RTS.RTSAttributeSet:MaxHealth")))) 1.0)
      (`SceneComponent.SetVisibility` _healthwidget false true)
      (else
        (`SceneComponent.SetVisibility` _healthwidget true true)))))

(fn `UpdateFogReveal`
  (bind _returnvalue (`self.K2_GetActorLocation`))
  (if (`self.bIsPlayersUnit`)
    (bind _outhit (`KismetSystemLibrary.LineTraceSingle` (+ _returnvalue (0.0 0.0 500.0)) (- _returnvalue (0.0 0.0 500.0)) "TraceTypeQuery4" true))
    (bind _uv (`GameplayStatics.FindCollisionUV` _outhit))
    (`MaterialInstanceDynamic.SetVectorParameterValue` (`self.FogMaterial`) "Location" (make `LinearColor` (`KismetMathLibrary.BreakVector2D` _uv) (`.Y` (`KismetMathLibrary.BreakVector2D` _uv)) 0.0 1.0))
    (`MaterialInstanceDynamic.SetVectorParameterValue` (`self.FogRevealMaterial`) "Location" (make `LinearColor` (`KismetMathLibrary.BreakVector2D` _uv) (`.Y` (`KismetMathLibrary.BreakVector2D` _uv)) 0.0 1.0))
    (`KismetRenderingLibrary.DrawMaterialToRenderTarget` "/Game/Blueprints/Fog/FogRender.FogRender" (`self.FogMaterial`))
    (`KismetRenderingLibrary.DrawMaterialToRenderTarget` "/Game/Blueprints/Fog/FogRevealRender.FogRevealRender" (`self.FogRevealMaterial`))))

(fn `UpdateHealthBarPercentage`
  (bind _abilitysystemcomponent (`self.AbilitySystemComponent`))
  (if (`self.bIsAlive`)
    (`ProgressBar.SetPercent` (`/Game/Blueprints/Widgets/WBP_HealthBar.ProgressBar_0` (`self.As WBP Health Bar`)) (/ (`.ReturnValue` (`AbilitySystemBlueprintLibrary.GetFloatAttributeFromAbilitySystemComponent` _abilitysystemcomponent (struct :`AttributeName` "Health" :`Attribute` "/Script/RTS.RTSAttributeSet:Health"))) (`.ReturnValue` (`AbilitySystemBlueprintLibrary.GetFloatAttributeFromAbilitySystemComponent` _abilitysystemcomponent (struct :`AttributeName` "MaxHealth" :`Attribute` "/Script/RTS.RTSAttributeSet:MaxHealth")))))))

(fn `UserConstructionScript`
  (`parent.UserConstructionScript`)
  (`self.SetFriendFoeDecal`)
  (`self.SetFriendFoeSprite`)
  (`PrimitiveComponent.SetVisibleInSceneCaptureOnly` (`self.PaperSprite`) true))