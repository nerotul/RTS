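; Base unit Blueprint that handles health bar display, friend/foe decal and fog-of-war reveal.
; Construction sets the decal; BeginPlay links the health widget, enables animation budgeting and clears the fog render targets.
; While alive, player units trace vertically each tick and draw fog materials into both targets at the hit UV.
; Health changes update the bar from Ability System attributes; health and sight events hide it at full health for living, enemy-sighted units.
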(event `self.ReceiveBeginPlay`
  (bind _aswbp_health_bar (cast `/Game/Blueprints/Widgets/WBP_HealthBar` (`WidgetComponent.GetUserWidgetObject` (`self.HealthWidget`))))
  (bind _output_get (set `self.As WBP Health Bar` _aswbp_health_bar))
  (set `/Game/Blueprints/Widgets/WBP_HealthBar.Owner` self _output_get)
  (`AnimationBudgetBlueprintLibrary.EnableAnimationBudget` true)
  (`self.InitFogReveal`))

(event `self.ReceiveTick`
  (params (DeltaSeconds :type "Float (single-precision)"))
  (if (`self.bIsAlive`)
    (`self.UpdateFogReveal`)))

(event `self.OnHealthChanged`
  (`self.UpdateHealthBarPercentage`)
  (`self.TryToggleHealthWidgetVisibility`))

(event `self.OnInEnemySight`
  (`self.TryToggleHealthWidgetVisibility`))

(fn `InitFogReveal`
  (bind _returnvalue (`KismetMaterialLibrary.CreateDynamicMaterialInstance` "/Game/Blueprints/Fog/M_FogMaterial.M_FogMaterial"))
  (set `self.FogMaterial` _returnvalue)
  (bind _returnvalue_2 (`KismetMaterialLibrary.CreateDynamicMaterialInstance` "/Game/Blueprints/Fog/M_FogRevealMaterial.M_FogRevealMaterial"))
  (set `self.FogRevealMaterial` _returnvalue_2)
  (`KismetRenderingLibrary.ClearRenderTarget2D` "/Game/Blueprints/Fog/FogRender.FogRender")
  (`KismetRenderingLibrary.ClearRenderTarget2D` "/Game/Blueprints/Fog/FogRevealRender.FogRevealRender")
  (`MaterialInstanceDynamic.SetScalarParameterValue` (`self.FogMaterial`) "Size" (`self.FogRevealCoeff`))
  (`MaterialInstanceDynamic.SetScalarParameterValue` (`self.FogRevealMaterial`) "Size" (`self.FogRevealCoeff`)))

(fn `TryToggleHealthWidgetVisibility`
  (bind _abilitysystemcomponent (`self.AbilitySystemComponent`))
  (bind _healthwidget (`self.HealthWidget`))
  (if (and (`self.bIsAlive`) (`self.bIsUnitInEnemySight`))
    (if (== (/ (`.ReturnValue` (`AbilitySystemBlueprintLibrary.GetFloatAttributeFromAbilitySystemComponent` _abilitysystemcomponent (struct :`AttributeName` "Health" :`Attribute` "/Script/RTS.RTSAttributeSet:Health"))) (`.ReturnValue` (`AbilitySystemBlueprintLibrary.GetFloatAttributeFromAbilitySystemComponent` _abilitysystemcomponent (struct :`AttributeName` "MaxHealth" :`Attribute` "/Script/RTS.RTSAttributeSet:MaxHealth")))) 1.0)
      (`SceneComponent.SetVisibility` _healthwidget false true)
      (else
        (`SceneComponent.SetVisibility` _healthwidget true true)))))

(fn `UpdateFogReveal`
  (bind _returnvalue (`self.K2_GetActorLocation`))
  (if (`self.bIsPlayersUnit`)
    (bind _outhit (`KismetSystemLibrary.LineTraceSingle` (+ _returnvalue (0.0 0.0 500.0)) (- _returnvalue (0.0 0.0 500.0)) "TraceTypeQuery4" true))
    (bind _uv (`GameplayStatics.FindCollisionUV` _outhit))
    (`MaterialInstanceDynamic.SetVectorParameterValue` (`self.FogMaterial`) "Location" (make `LinearColor` (`KismetMathLibrary.BreakVector2D` _uv) (`.Y` (`KismetMathLibrary.BreakVector2D` _uv)) 0.0 1.0))
    (`MaterialInstanceDynamic.SetVectorParameterValue` (`self.FogRevealMaterial`) "Location" (make `LinearColor` (`KismetMathLibrary.BreakVector2D` _uv) (`.Y` (`KismetMathLibrary.BreakVector2D` _uv)) 0.0 1.0))
    (`KismetRenderingLibrary.DrawMaterialToRenderTarget` "/Game/Blueprints/Fog/FogRender.FogRender" (`self.FogMaterial`))
    (`KismetRenderingLibrary.DrawMaterialToRenderTarget` "/Game/Blueprints/Fog/FogRevealRender.FogRevealRender" (`self.FogRevealMaterial`))))

(fn `UpdateHealthBarPercentage`
  (bind _abilitysystemcomponent (`self.AbilitySystemComponent`))
  (if (`self.bIsAlive`)
    (`ProgressBar.SetPercent` (`/Game/Blueprints/Widgets/WBP_HealthBar.ProgressBar_0` (`self.As WBP Health Bar`)) (/ (`.ReturnValue` (`AbilitySystemBlueprintLibrary.GetFloatAttributeFromAbilitySystemComponent` _abilitysystemcomponent (struct :`AttributeName` "Health" :`Attribute` "/Script/RTS.RTSAttributeSet:Health"))) (`.ReturnValue` (`AbilitySystemBlueprintLibrary.GetFloatAttributeFromAbilitySystemComponent` _abilitysystemcomponent (struct :`AttributeName` "MaxHealth" :`Attribute` "/Script/RTS.RTSAttributeSet:MaxHealth")))))))

(fn `UserConstructionScript`
  (`self.SetFriendFoeDecal`))