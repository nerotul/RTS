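; BP_Unit is an RTS unit that can be targeted by right-click and can damage other actors.
; Right-clicking a non-player unit makes it the target of every unit in the player controller's selection, writing a random navigable point nearby and an action enum to their blackboards.
; Attack applies damage to the stored target, while taking damage only prints a debug message.
; The construction script sets a friend-or-foe decal.
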(event `self.ReceiveActorOnClicked`
  (params (ButtonPressed :type "Key Structure"))
  (if (and (not (`self.bIsPlayersUnit`)) (== ButtonPressed "RightMouseButton"))
    (bind _asbp_rtsplayer_controller (cast `/Game/Blueprints/BP_RTSPlayerController` (`GameplayStatics.GetPlayerController` 0)))
    (for _array_element (`RTSPlayerControllerBase.UnitSelection` _asbp_rtsplayer_controller)
      (set `UnitBase.TargetActor` self _array_element)
      (bind _returnvalue (`AIBlueprintHelperLibrary.GetBlackboard` _array_element))
      (`BlackboardComponent.SetValueAsVector` _returnvalue "TargetLocation" (`NavigationSystemV1.K2_GetRandomLocationInNavigableRadius` (`self.K2_GetActorLocation`) 50.0 null null))
      (`BlackboardComponent.SetValueAsEnum` _returnvalue "ActionEnum" (`self.Enum Value`)))))

(event `Attack`
  (`GameplayStatics.ApplyDamage` (`self.TargetActor`) (`self.Base Damage`) (`self.GetController`) self))

(event `self.ReceiveAnyDamage`
  (params (Damage :type "Float (single-precision)") (DamageType :type "DamageType Object Reference") (InstigatedBy :type "Controller Object Reference") (DamageCauser :type "Actor Object Reference"))
  (`KismetSystemLibrary.PrintString` "OUCH!"))

(fn `UserConstructionScript`
  (`self.SetFriendFoeDecal`))